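; BP_FT_SimpleJetpack is a cosmetic jetpack that shows left and right Niagara fire effects while its target character jumps.
; Init stores the character and start delay, then assigns the Niagara asset to both emitters.
; JumpStart fires the effects immediately if the jump count is non-zero, otherwise after a cancelable timer delay.
; JumpEnd cancels that timer, switching both effects off whether it was pending or already stopped.
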(event Custom|JetpackActive_Event
  (Components|Activation|SetActive (Variables|Default|GetNS_Fire_L) true false))

(event EventJumpStart
  (bind _ns_fire_l (Variables|Default|GetNS_Fire_L))
  (if (!= (Variables|/Script/Engine.Character|GetJumpCurrentCount (Variables|Default|GetTargetChara)) 0)
    (Components|Activation|SetActive _ns_fire_l true false)
    (else
      (Utilities|CancelableSetTimerbyEvent (delegate Custom|JetpackActive_Event) (Variables|Default|GetStartFXDelay) false
        (:OnCanceled
          _)
        (:OnAlreadyStopped
          _))
      (Components|Activation|SetActive _ns_fire_l false false))))

(event EventJumpEnd
  (Utilities|CancelableSetTimerbyEvent (delegate Custom|JetpackActive_Event) (Variables|Default|GetStartFXDelay) false) ; enters at OnCancel
)

(event EventInit
  (params (TargetCharacter :type Character%20Object%20Reference) (JetpackFX :type Niagara%20System%20Object%20Reference) (StartFXDelay :type Float%20%28double-precision%29))
  (bind _output_get (Variables|Default|SetTargetChara TargetCharacter))
  (Variables|Default|SetTargetCharaMesh (Variables|/Script/Engine.Character|GetMesh _output_get))
  (CallFunction|SetEffect JetpackFX)
  (Variables|Default|SetStartFXDelay StartFXDelay))

(event EventSetEffect
  (params (JetpackFX :type Niagara%20System%20Object%20Reference))
  (Class|NiagaraComponent|SetAsset (Variables|Default|GetNS_Fire_L) JetpackFX true)
  (Class|NiagaraComponent|SetAsset (Variables|Default|GetNS_Fire_R) JetpackFX true))

(fn ConstructionScript)