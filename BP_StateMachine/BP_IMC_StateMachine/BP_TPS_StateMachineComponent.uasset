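; A state machine component for a third-person character, switching between landing, on-air, zip line, sword-swing and Tarzan states.
; Awake constructs one object per state, and Initialize sets the starting state, passes the character to each state, then enters the start state.
; TransitionTo exits the current state and enters the next, while Update forwards to the current state.
; Invalid state instances print an error and halt the init chain.
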(fn GetCurrentState
  (return (Variables|Default|GetCurrentState)))

(fn Awake
  (bind _returnvalue (Game|ConstructObjectfromClass self "/Game/MyContent/FT/BP_StateMachine/BP_IMC_StateMachine/BP_TPS_States/BP_TPS_LandingState.BP_TPS_LandingState_C"))
  (Variables|Default|SetLandingState _returnvalue)
  (bind _returnvalue_2 (Game|ConstructObjectfromClass self "/Game/MyContent/FT/BP_StateMachine/BP_IMC_StateMachine/BP_TPS_States/BP_TPS_OnAirState.BP_TPS_OnAirState_C"))
  (Variables|Default|SetOnAirState _returnvalue_2)
  (bind _returnvalue_3 (Game|ConstructObjectfromClass self "/Game/MyContent/FT/BP_StateMachine/BP_IMC_StateMachine/BP_TPS_States/BP_TPS_OnZipLineState.BP_TPS_OnZipLineState_C"))
  (Variables|Default|SetOnZipLineState _returnvalue_3)
  (bind _returnvalue_4 (Game|ConstructObjectfromClass self "/Game/MyContent/FT/BP_StateMachine/BP_IMC_StateMachine/BP_TPS_States/BP_TPS_SwingSwordState.BP_TPS_SwingSwordState_C"))
  (Variables|Default|SetSwingingSwordState _returnvalue_4)
  (bind _returnvalue_5 (Game|ConstructObjectfromClass self "/Game/MyContent/FT/BP_StateMachine/BP_IMC_StateMachine/BP_TPS_States/BP_TPS_OnTarzanState.BP_TPS_OnTarzanState_C"))
  (Variables|Default|SetOnTarzanState _returnvalue_5))

(fn Initialize
  (params (StartingState :type BPI%20State%20Interface) (MyThirdPersonCharacter :type BP%20My%20Third%20Person%20Character%20Object%20Reference))
  (Utilities|FlowControl|Sequence
    (:then_0
      (Variables|Default|SetCurrentState StartingState)
      (LocalVariables|SetMyTPSChara MyThirdPersonCharacter))
    (:then_1
      (bind _landingstate (Variables|Default|GetLandingState)
        (:then
          (Default|Init _landingstate (LocalVariables|GetMyTPSChara))
          (bind _onairstate (Variables|Default|GetOnAirState)
            (:then
              (Default|Init _onairstate (LocalVariables|GetMyTPSChara))
              (bind _swingingswordstate (Variables|Default|GetSwingingSwordState)
                (:then
                  (Default|Init _swingingswordstate (LocalVariables|GetMyTPSChara))
                  (bind _onziplinestate (Variables|Default|GetOnZipLineState)
                    (:then
                      (Default|Init _onziplinestate (LocalVariables|GetMyTPSChara))
                      (bind _ontarzanstate (Variables|Default|GetOnTarzanState)
                        (:then
                          (Default|Init _ontarzanstate (LocalVariables|GetMyTPSChara)))
                        (:else
                          (Development|PrintString "OnTarzan State Instance is Null Exeption" true true "(R=1.000000,G=0.220031,B=0.070112,A=1.000000)" 2.0 "Error"))))
                    (:else
                      (Development|PrintString "OnZipLine State Instance is Null Exeption" true true "(R=1.000000,G=0.220031,B=0.070112,A=1.000000)" 2.0 "Error"))))
                (:else
                  (Development|PrintString "SwingingSword State Instance is Null Exeption" true true "(R=1.000000,G=0.220031,B=0.070112,A=1.000000)" 2.0 "Error"))))
            (:else
              (Development|PrintString "OnAir State Instance is Null Exeption" true true "(R=1.000000,G=0.220031,B=0.070112,A=1.000000)" 2.0 "Error"))))
        (:else
          (Development|PrintString "Landing State Instance is Null Exeption" true true "(R=1.000000,G=0.220031,B=0.070112,A=1.000000)" 2.0 "Error"))))
    (:then_2
      (Default|Enter (Variables|Default|GetCurrentState)))))

(fn Transitionto
  (params (NextState :type BPI%20State%20Interface))
  (Default|Exit (Variables|Default|GetCurrentState))
  (bind _output_get (Variables|Default|SetCurrentState NextState))
  (Default|Enter _output_get))

(fn Update
  (Default|Update (Variables|Default|GetCurrentState)))