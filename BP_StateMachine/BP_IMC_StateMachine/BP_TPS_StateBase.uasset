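; Base state class for the third-person character's state machine, covering movement modes like airborne, landing, sword swinging, zip line and Tarzan.
; Enter and Exit add and remove the state's Enhanced Input mapping context, so each state carries its own controls.
; Update checks character flags and falling status behind per-state CanTransientTo booleans, then asks the state machine component to transition.
; Init caches the owning character, and GetStateString exposes the state name.
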(event EventUpdate
  (bind _mytpschara (Variables|Default|GetMyTPSChara))
  (bind _mytpschara_2 (Variables|Default|GetMyTPSChara))
  (bind _mytpschara_3 (Variables|Default|GetMyTPSChara))
  (bind _mytpschara_4 (Variables|Default|GetMyTPSChara))
  (bind _mytpschara_5 (Variables|Default|GetMyTPSChara))
  (bind _mytpschara_6 (Variables|Default|GetMyTPSChara))
  (bind _bp_tps_statemachinecomponent (Variables|/Game/MyContent/BP_MyThirdPersonCharacter.BP_MyThirdPersonCharacter_C|GetBP_TPS_StateMachineComponent _mytpschara))
  (bind _bp_tps_statemachinecomponent_2 (Variables|/Game/MyContent/BP_MyThirdPersonCharacter.BP_MyThirdPersonCharacter_C|GetBP_TPS_StateMachineComponent _mytpschara_3))
  (bind _bp_tps_statemachinecomponent_3 (Variables|/Game/MyContent/BP_MyThirdPersonCharacter.BP_MyThirdPersonCharacter_C|GetBP_TPS_StateMachineComponent _mytpschara_2))
  (bind _bp_tps_statemachinecomponent_4 (Variables|/Game/MyContent/BP_MyThirdPersonCharacter.BP_MyThirdPersonCharacter_C|GetBP_TPS_StateMachineComponent _mytpschara_4))
  (bind _bp_tps_statemachinecomponent_5 (Variables|/Game/MyContent/BP_MyThirdPersonCharacter.BP_MyThirdPersonCharacter_C|GetBP_TPS_StateMachineComponent _mytpschara_5))
  (bind _bp_tps_statemachinecomponent_6 (Variables|/Game/MyContent/BP_MyThirdPersonCharacter.BP_MyThirdPersonCharacter_C|GetBP_TPS_StateMachineComponent _mytpschara_6))
  (Utilities|FlowControl|Sequence
    (:then_0
      (if (Variables|Default|GetCanTransientToOnAir)
        (if (AI|Components|NavMovement|IsFalling (Variables|/Script/Engine.Character|GetCharacterMovement (Variables|Default|GetMyTPSChara)))
          (Default|Transitionto _bp_tps_statemachinecomponent (Variables|/Game/MyContent/FT/BP_StateMachine/BP_IMC_StateMachine/BP_TPS_StateMachineComponent.BP_TPS_StateMachineComponent_C|GetOnAirState _bp_tps_statemachinecomponent)))))
    (:then_1
      (if (Variables|Default|GetCanTransientToSwingSword)
        (if (Variables|/Game/MyContent/BP_MyThirdPersonCharacter.BP_MyThirdPersonCharacter_C|GetIsSwingingSword (Variables|Default|GetMyTPSChara))
          (Default|Transitionto _bp_tps_statemachinecomponent (Variables|/Game/MyContent/FT/BP_StateMachine/BP_IMC_StateMachine/BP_TPS_StateMachineComponent.BP_TPS_StateMachineComponent_C|GetSwingingSwordState _bp_tps_statemachinecomponent)))))
    (:then_2
      (if (Variables|Default|GetCanTransientToOnZipLine)
        (if (Variables|/Game/MyContent/BP_MyThirdPersonCharacter.BP_MyThirdPersonCharacter_C|GetIsOnZipLine (Variables|Default|GetMyTPSChara))
          (Default|Transitionto _bp_tps_statemachinecomponent (Variables|/Game/MyContent/FT/BP_StateMachine/BP_IMC_StateMachine/BP_TPS_StateMachineComponent.BP_TPS_StateMachineComponent_C|GetOnZipLineState _bp_tps_statemachinecomponent)))))
    (:then_3
      (if (Variables|Default|GetCanTransientToOnLand)
        (if (not (AI|Components|NavMovement|IsFalling (Variables|/Script/Engine.Character|GetCharacterMovement (Variables|Default|GetMyTPSChara))))
          (Default|Transitionto _bp_tps_statemachinecomponent_2 (Variables|/Game/MyContent/FT/BP_StateMachine/BP_IMC_StateMachine/BP_TPS_StateMachineComponent.BP_TPS_StateMachineComponent_C|GetLandingState _bp_tps_statemachinecomponent_2)))))
    (:then_4
      (if (Variables|Default|GetCanTransientToSwingSwordEnd)
        (if (not (Variables|/Game/MyContent/BP_MyThirdPersonCharacter.BP_MyThirdPersonCharacter_C|GetIsSwingingSword (Variables|Default|GetMyTPSChara)))
          (Default|Transitionto _bp_tps_statemachinecomponent_4 (Variables|/Game/MyContent/FT/BP_StateMachine/BP_IMC_StateMachine/BP_TPS_StateMachineComponent.BP_TPS_StateMachineComponent_C|GetLandingState _bp_tps_statemachinecomponent_4)))))
    (:then_5
      (if (Variables|Default|GetCanTransientToZipLineOff)
        (if (not (Variables|/Game/MyContent/BP_MyThirdPersonCharacter.BP_MyThirdPersonCharacter_C|GetIsOnZipLine (Variables|Default|GetMyTPSChara)))
          (Default|Transitionto _bp_tps_statemachinecomponent_5 (Variables|/Game/MyContent/FT/BP_StateMachine/BP_IMC_StateMachine/BP_TPS_StateMachineComponent.BP_TPS_StateMachineComponent_C|GetOnAirState _bp_tps_statemachinecomponent_5)))))
    (:then_6
      (if (Variables|Default|GetCanTransientToTarzanOff)
        (if (not (Variables|/Game/MyContent/BP_MyThirdPersonCharacter.BP_MyThirdPersonCharacter_C|GetIsOnTarzan (Variables|Default|GetMyTPSChara)))
          (Default|Transitionto _bp_tps_statemachinecomponent_6 (Variables|/Game/MyContent/FT/BP_StateMachine/BP_IMC_StateMachine/BP_TPS_StateMachineComponent.BP_TPS_StateMachineComponent_C|GetOnAirState _bp_tps_statemachinecomponent_6)))))
    (:then_7
      (if (Variables|Default|GetCanTransientToTarzanOn)
        (if (Variables|/Game/MyContent/BP_MyThirdPersonCharacter.BP_MyThirdPersonCharacter_C|GetIsOnTarzan (Variables|Default|GetMyTPSChara))
          (Default|Transitionto _bp_tps_statemachinecomponent_3 (Variables|/Game/MyContent/FT/BP_StateMachine/BP_IMC_StateMachine/BP_TPS_StateMachineComponent.BP_TPS_StateMachineComponent_C|GetOnTarzanState _bp_tps_statemachinecomponent_3)))))))

(event EventEnter
  (CallFunction|AddMappingContext (Variables|Default|GetMappingContext)))

(event EventExit
  (CallFunction|RemoveMappingContext (Variables|Default|GetMappingContext)))

(fn Init
  (params (MyThirdPersonCharacter :type BP%20My%20Third%20Person%20Character%20Object%20Reference))
  (Variables|Default|SetMyTPSChara MyThirdPersonCharacter))

(fn AddMappingContext
  (params (MappingContext :type Input%20Mapping%20Context%20Object%20Reference))
  (bind _mytpschara (Variables|Default|GetMyTPSChara))
  (bind _playercontroller (Variables|/Game/MyContent/BP_MyThirdPersonCharacter.BP_MyThirdPersonCharacter_C|GetPlayerController _mytpschara))
  (bind _returnvalue (PlayerController|LocalPlayerSubsystems|GetEnhancedInputLocalPlayerSubsystem _playercontroller))
  (Utilities|IsValid _returnvalue
    (:Is%20Valid
      (Input|AddMappingContext _returnvalue MappingContext 2 "(bIgnoreAllPressedKeysUntilRelease=True,bForceImmediately=False,bNotifyUserSettings=False)"))))

(fn RemoveMappingContext
  (params (MappingContext :type Input%20Mapping%20Context%20Object%20Reference))
  (bind _mytpschara (Variables|Default|GetMyTPSChara))
  (bind _playercontroller (Variables|/Game/MyContent/BP_MyThirdPersonCharacter.BP_MyThirdPersonCharacter_C|GetPlayerController _mytpschara))
  (bind _returnvalue (PlayerController|LocalPlayerSubsystems|GetEnhancedInputLocalPlayerSubsystem _playercontroller))
  (Utilities|IsValid _returnvalue
    (:Is%20Valid
      (Input|RemoveMappingContext _returnvalue MappingContext "(bIgnoreAllPressedKeysUntilRelease=True,bForceImmediately=False,bNotifyUserSettings=False)"))))

(fn GetStateString
  (return (Utilities|String|ToString(Name) (Variables|Default|GetStatusName))))