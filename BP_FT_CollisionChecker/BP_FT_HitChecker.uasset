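; BP_FT_HitChecker is a debug checker that diagnoses hit collision setup between two actors' primitive components.
; CheckOverlap_Event finds components tagged OverlapHitA and OverlapHitB on ActorA and ActorB, runs CheckHitAB, then binds both hit events to print messages.
; CheckHitAB prints failures in mutual channel responses, physics collision enablement and overlap-event generation, though A's overlap check is hardwired to pass.
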(event Custom|CheckOverlap_Event
  (bind _actora (Variables|Default|GetActorA))
  (bind _actorb (Variables|Default|GetActorB))
  (bind _returnvalue (Actor|GetComponentsbyTag _actorb "/Script/Engine.PrimitiveComponent" "OverlapHitB"))
  (bind _returnvalue_2 (Actor|GetComponentsbyTag _actora "/Script/Engine.PrimitiveComponent" "OverlapHitA"))
  (bind _output (Utilities|Array|Get(acopy) _returnvalue))
  (bind _output_2 (Utilities|Array|Get(acopy) _returnvalue_2))
  (Utilities|IsValid _output_2
    (:Is%20Valid
      (Utilities|IsValid _output
        (:Is%20Valid
          (CallFunction|CheckHitAB _output_2 _output)
          (Collision|BindEventtoOnComponentHit _output_2 (delegate Custom|AOnHitEvent))
          (Collision|BindEventtoOnComponentHit _output (delegate Custom|BOnHitEvent)))
        (:Is%20Not%20Valid
          (Development|PrintString "Invalid HitCheckerB"))))
    (:Is%20Not%20Valid
      (Development|PrintString "Invalid HitCheckerA"))))

(event Custom|BOnHitEvent
  (params (HitComponent :type Primitive%20Component%20Object%20Reference) (OtherActor :type Actor%20Object%20Reference) (OtherComp :type Primitive%20Component%20Object%20Reference) (NormalImpulse :type Vector) (Hit :type Hit%20Result%20Structure%20%28by%20ref%29))
  (Development|PrintString "B Hit Event Occured!!!!" true true "(R=0.088914,G=0.529822,B=1.000000,A=1.000000)"))

(event Custom|AOnHitEvent
  (params (HitComponent :type Primitive%20Component%20Object%20Reference) (OtherActor :type Actor%20Object%20Reference) (OtherComp :type Primitive%20Component%20Object%20Reference) (NormalImpulse :type Vector) (Hit :type Hit%20Result%20Structure%20%28by%20ref%29))
  (Development|PrintString "A Hit Event Occured!!!!" true true "(R=0.088914,G=0.529822,B=1.000000,A=1.000000)"))

(fn ConstructionScript)

(fn CheckHitAB
  (params (PrimitiveComponentA :type Primitive%20Component%20Object%20Reference) (PrimitiveComponentB :type Primitive%20Component%20Object%20Reference))
  (LocalVariables|SetPrimA PrimitiveComponentA)
  (LocalVariables|SetPrimB PrimitiveComponentB)
  (LocalVariables|SetObjectTypeA (Collision|GetCollisionObjectType (LocalVariables|GetPrimA)))
  (LocalVariables|SetObjectTypeB (Collision|GetCollisionObjectType (LocalVariables|GetPrimB)))
  (bind _output_get (LocalVariables|SetACollisionResponcesToB (Collision|GetCollisionResponsetoChannel (LocalVariables|GetPrimA) (LocalVariables|GetObjectTypeB))))
  (LocalVariables|SetAIgnoreB (Utilities|Enum|Equal(Enum) _output_get "ECR_Ignore"))
  (bind _output_get_2 (LocalVariables|SetBCollisionResponcesToA (Collision|GetCollisionResponsetoChannel (LocalVariables|GetPrimB) (LocalVariables|GetObjectTypeA))))
  (LocalVariables|SetBIgnoreA (Utilities|Enum|Equal(Enum) _output_get_2 "ECR_Ignore"))
  (if (LocalVariables|GetAIgnoreB)
    (Development|PrintString "A Ignore B." true true "(R=1.000000,G=0.112334,B=0.000000,A=1.000000)"))
  (if (LocalVariables|GetBIgnoreA)
    (Development|PrintString "B Ignore A." true true "(R=1.000000,G=0.112334,B=0.000000,A=1.000000)"))
  (bind _output_get_3 (LocalVariables|SetPhysicsCollisionAble_A (or (Utilities|Enum|Equal(Enum) (Collision|GetCollisionEnabled (LocalVariables|GetPrimA)) "PhysicsOnly") (Utilities|Enum|Equal(Enum) (Collision|GetCollisionEnabled (LocalVariables|GetPrimA)) "QueryAndPhysics"))))
  (bind _output_get_4 (LocalVariables|SetPhysicsCollisionAble_B (or (Utilities|Enum|Equal(Enum) (Collision|GetCollisionEnabled (LocalVariables|GetPrimB)) "PhysicsOnly") (Utilities|Enum|Equal(Enum) (Collision|GetCollisionEnabled (LocalVariables|GetPrimB)) "QueryAndPhysics"))))
  (if (and _output_get_3 _output_get_4)
    _
    (else
      (if (not (LocalVariables|GetPhysicsCollisionAble_A))
        (Development|PrintString "A is Not Query Collisionable" true true "(R=1.000000,G=0.112334,B=0.000000,A=1.000000)"))
      (if (not (LocalVariables|GetPhysicsCollisionAble_B))
        (Development|PrintString "B is Not Query Collisionable" true true "(R=1.000000,G=0.112334,B=0.000000,A=1.000000)"))))
  (bind _output_get_5 (LocalVariables|SetABlockB (Utilities|Enum|Equal(Enum) (LocalVariables|GetACollisionResponcesToB) "ECR_Block")))
  (bind _output_get_6 (LocalVariables|SetBBlockA (Utilities|Enum|Equal(Enum) (LocalVariables|GetBCollisionResponcesToA) "ECR_Block")))
  (if (and _output_get_5 _output_get_6)
    _
    (else
      (if (not (LocalVariables|GetABlockB))
        (Development|PrintString "A Not Block B" true true "(R=1.000000,G=0.112334,B=0.000000,A=1.000000)"))
      (if (not (LocalVariables|GetBBlockA))
        (Development|PrintString "B Not Block A" true true "(R=1.000000,G=0.112334,B=0.000000,A=1.000000)"))))
  (if true
    _
    (else
      (Development|PrintString "A Not Generate Overlap Events" true true "(R=1.000000,G=0.112334,B=0.000000,A=1.000000)")))
  (if (not (Variables|/Script/Engine.PrimitiveComponent|GetbGenerateOverlapEvents (LocalVariables|GetPrimB)))
    (Development|PrintString "B Not Generate Overlap Events" true true "(R=1.000000,G=0.112334,B=0.000000,A=1.000000)")))