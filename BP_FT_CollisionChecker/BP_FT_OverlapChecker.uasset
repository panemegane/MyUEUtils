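; Debug Blueprint that diagnoses why two actors' components may fail to generate overlap events.
; CheckOverlap_Event finds the primitive components tagged OverlapCheckerA and OverlapCheckerB on ActorA and ActorB.
; CheckOverlapAB compares their channel responses, query collision and Generate Overlap Events settings, printing each problem found.
; It also binds both components' begin-overlap events to print when an overlap actually fires.
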(event Custom|CheckOverlap_Event
  (bind _actora (Variables|Default|GetActorA))
  (bind _actorb (Variables|Default|GetActorB))
  (bind _returnvalue (Actor|GetComponentsbyTag _actorb "/Script/Engine.PrimitiveComponent" "OverlapCheckerB"))
  (bind _returnvalue_2 (Actor|GetComponentsbyTag _actora "/Script/Engine.PrimitiveComponent" "OverlapCheckerA"))
  (bind _output (Utilities|Array|Get(acopy) _returnvalue))
  (bind _output_2 (Utilities|Array|Get(acopy) _returnvalue_2))
  (Utilities|IsValid _output_2
    (:Is%20Valid
      (Utilities|IsValid _output
        (:Is%20Valid
          (CallFunction|CheckOverlapAB _output_2 _output)
          (Collision|BindEventtoOnComponentBeginOverlap _output_2 (delegate Custom|OnComponentBeginOverlap_EventA))
          (Collision|BindEventtoOnComponentBeginOverlap _output (delegate Custom|OnComponentBeginOverlap_EventB)))
        (:Is%20Not%20Valid
          (Development|PrintString "Invalid OverlapCheckerB"))))
    (:Is%20Not%20Valid
      (Development|PrintString "Invalid OverlapCheckerA"))))

(event Custom|OnComponentBeginOverlap_EventB
  (params (OverlappedComponent :type Primitive%20Component%20Object%20Reference) (OtherActor :type Actor%20Object%20Reference) (OtherComp :type Primitive%20Component%20Object%20Reference) (OtherBodyIndex :type Integer) (bFromSweep :type Boolean) (SweepResult :type Hit%20Result%20Structure%20%28by%20ref%29))
  (Development|PrintString "B Overlap Event Occured!!!!" true true "(R=0.088914,G=0.529822,B=1.000000,A=1.000000)"))

(event Custom|OnComponentBeginOverlap_EventA
  (params (OverlappedComponent :type Primitive%20Component%20Object%20Reference) (OtherActor :type Actor%20Object%20Reference) (OtherComp :type Primitive%20Component%20Object%20Reference) (OtherBodyIndex :type Integer) (bFromSweep :type Boolean) (SweepResult :type Hit%20Result%20Structure%20%28by%20ref%29))
  (Development|PrintString "A Overlap Event Occured!!!!" true true "(R=0.088914,G=0.529822,B=1.000000,A=1.000000)"))

(fn ConstructionScript)

(fn CheckOverlapAB
  (params (PrimitiveComponentA :type Primitive%20Component%20Object%20Reference) (PrimitiveComponentB :type Primitive%20Component%20Object%20Reference))
  (LocalVariables|SetPrimA PrimitiveComponentA)
  (LocalVariables|SetPrimB PrimitiveComponentB)
  (LocalVariables|SetObjectTypeA (Collision|GetCollisionObjectType (LocalVariables|GetPrimA)))
  (LocalVariables|SetObjectTypeB (Collision|GetCollisionObjectType (LocalVariables|GetPrimB)))
  (bind _output_get (LocalVariables|SetACollisionResponcesToB (Collision|GetCollisionResponsetoChannel (LocalVariables|GetPrimA) (LocalVariables|GetObjectTypeB))))
  (LocalVariables|SetAIgnoreB (Utilities|Enum|Equal(Enum) _output_get "ECR_Ignore"))
  (bind _output_get_2 (LocalVariables|SetBCollisionResponcesToA (Collision|GetCollisionResponsetoChannel (LocalVariables|GetPrimB) (LocalVariables|GetObjectTypeA))))
  (LocalVariables|SetBIgnoreA (Utilities|Enum|Equal(Enum) _output_get_2 "ECR_Ignore"))
  (if (LocalVariables|GetAIgnoreB)
    (Development|PrintString "A Ignore B." true true "(R=1.000000,G=0.112334,B=0.000000,A=1.000000)"))
  (if (LocalVariables|GetBIgnoreA)
    (Development|PrintString "B Ignore A." true true "(R=1.000000,G=0.112334,B=0.000000,A=1.000000)"))
  (bind _output_get_3 (LocalVariables|SetQueryCollisionAble_A (Math|Boolean|ORBoolean (Utilities|Enum|Equal(Enum) (Collision|GetCollisionEnabled (LocalVariables|GetPrimA)) "QueryAndProbe") (Utilities|Enum|Equal(Enum) (Collision|GetCollisionEnabled (LocalVariables|GetPrimA)) "QueryAndPhysics") (Utilities|Enum|Equal(Enum) (Collision|GetCollisionEnabled (LocalVariables|GetPrimA)) "QueryOnly"))))
  (bind _output_get_4 (LocalVariables|SetQueryCollisionAble_B (Math|Boolean|ORBoolean (Utilities|Enum|Equal(Enum) (Collision|GetCollisionEnabled (LocalVariables|GetPrimB)) "QueryAndProbe") (Utilities|Enum|Equal(Enum) (Collision|GetCollisionEnabled (LocalVariables|GetPrimB)) "QueryAndPhysics") (Utilities|Enum|Equal(Enum) (Collision|GetCollisionEnabled (LocalVariables|GetPrimB)) "QueryOnly"))))
  (if (and _output_get_3 _output_get_4)
    _
    (else
      (if (not (LocalVariables|GetQueryCollisionAble_A))
        (Development|PrintString "A is Not Query Collisionable" true true "(R=1.000000,G=0.112334,B=0.000000,A=1.000000)"))
      (if (not (LocalVariables|GetQueryCollisionAble_B))
        (Development|PrintString "B is Not Query Collisionable" true true "(R=1.000000,G=0.112334,B=0.000000,A=1.000000)"))))
  (bind _output_get_5 (LocalVariables|SetAOverlapB (Utilities|Enum|Equal(Enum) (LocalVariables|GetACollisionResponcesToB) "ECR_Overlap")))
  (bind _output_get_6 (LocalVariables|SetBOverlapA (Utilities|Enum|Equal(Enum) (LocalVariables|GetBCollisionResponcesToA) "ECR_Overlap")))
  (if (or _output_get_5 _output_get_6)
    _
    (elif (and (not (LocalVariables|GetAIgnoreB)) (not (LocalVariables|GetBIgnoreA)))
      (Development|PrintString "A and B Not overlap each other" true true "(R=1.000000,G=0.112334,B=0.000000,A=1.000000)")))
  (if (Variables|/Script/Engine.PrimitiveComponent|GetbGenerateOverlapEvents (LocalVariables|GetPrimA))
    _
    (else
      (Development|PrintString "A Not Generate Overlap Events" true true "(R=1.000000,G=0.112334,B=0.000000,A=1.000000)")))
  (if (not (Variables|/Script/Engine.PrimitiveComponent|GetbGenerateOverlapEvents (LocalVariables|GetPrimB)))
    (Development|PrintString "B Not Generate Overlap Events" true true "(R=1.000000,G=0.112334,B=0.000000,A=1.000000)")))