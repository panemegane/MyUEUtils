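; Timer actor component that counts elapsed time up or down toward a configurable limit.
; A state enum (PreStart, Started, Stopped, SpentExceed) gates Start and Stop, and Tick advances CurrentSpent only while Started.
; Crossing the limit clamps the value and enters SpentExceed, which fires the OnSpentExceeeded dispatcher.
; SetStat centralises transitions and mirrors the state into boolean flags, while InitTimer resets everything to PreStart.
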(event EventBeginPlay
  (CallFunction|SetStat "NewEnumerator0")
  (CallFunction|InitTimer (Variables|Default|GetIsIncreaseSpentMode) (Variables|Default|GetLimitSpent) 0.0))

(event EventTick
  (params (DeltaSeconds :type Float%20%28single-precision%29))
  (bind _output_get (Variables|Default|SetDeltaSeconds DeltaSeconds))
  (Variables|Default|SetTimeTime (+ _output_get (Variables|Default|GetTimeTime)))
  (switch Utilities|FlowControl|Switch|SwitchonE_FT_TimerStat (Variables|Default|GetStat)
    (:NewEnumerator1
      (if (Variables|Default|GetIsIncreaseSpentMode)
        (Variables|Default|SetCurrentSpent (+ (Variables|Default|GetDeltaSeconds) (Variables|Default|GetCurrentSpent)))
        (if (> (Variables|Default|GetCurrentSpent) (Variables|Default|GetLimitSpent))
          (Variables|Default|SetCurrentSpent (Variables|Default|GetLimitSpent) :!label _label)
          (CallFunction|SetStat "NewEnumerator3"))
        (else
          (Variables|Default|SetCurrentSpent (- (Variables|Default|GetCurrentSpent) (Variables|Default|GetDeltaSeconds)))
          (if (> (Variables|Default|GetLimitSpent) (Variables|Default|GetCurrentSpent))
            (goto _label)))))))

(fn InitTimer
  (params (IsIncreaseSpentMode :type Boolean) (LimitSpent :type Float%20%28double-precision%29) (CurrentSpent :type Float%20%28double-precision%29))
  (Variables|Default|SetCurrentSpent CurrentSpent)
  (Variables|Default|SetLimitSpent LimitSpent)
  (Variables|Default|SetIsIncreaseSpentMode IsIncreaseSpentMode)
  (CallFunction|SetStat "NewEnumerator0"))

(fn StartTimer
  (bind _stat (Variables|Default|GetStat))
  (if (or (Utilities|Enum|Equal(Enum) _stat "NewEnumerator0") (Utilities|Enum|Equal(Enum) _stat "NewEnumerator2"))
    (CallFunction|SetStat "NewEnumerator1")))

(fn StopTimer
  (if (Utilities|Enum|Equal(Enum) (Variables|Default|GetStat) "NewEnumerator1")
    (CallFunction|SetStat "NewEnumerator2")))

(fn SetStat
  (params (NewParam :type E_FT_TimerStat%20Enum :default "NewEnumerator0"))
  (bind _output_get (Variables|Default|SetStat NewParam))
  (switch Utilities|FlowControl|Switch|SwitchonE_FT_TimerStat _output_get
    (:NewEnumerator0
      _)
    (:NewEnumerator1
      _)
    (:NewEnumerator2
      _)
    (:NewEnumerator3
      (Default|CallOnSpentExceeeded)))
  (if (Utilities|Enum|Equal(Enum) (Variables|Default|GetStat) "NewEnumerator0")
    (Variables|Default|SetIsPreStart true)
    (else
      (Variables|Default|SetIsPreStart false)))
  (if (Utilities|Enum|Equal(Enum) (Variables|Default|GetStat) "NewEnumerator1")
    (Variables|Default|SetIsStarted true)
    (else
      (Variables|Default|SetIsStarted false)))
  (if (Utilities|Enum|Equal(Enum) (Variables|Default|GetStat) "NewEnumerator2")
    (Variables|Default|SetIsStopped true)
    (else
      (Variables|Default|SetIsStopped false)))
  (if (Utilities|Enum|Equal(Enum) (Variables|Default|GetStat) "NewEnumerator3")
    (Variables|Default|SetIsSpentExceeded true)
    (else
      (Variables|Default|SetIsSpentExceeded false))))