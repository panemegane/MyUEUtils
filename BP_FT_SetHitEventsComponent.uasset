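; Component that gives a static mesh begin, stay and end hit events.
; Init attaches a supplied mesh component to the target as a scaled, query-only copy of its mesh that overlaps all channels.
; Overlaps count as hits only when the other component blocks the copy's object type; those actors are tracked in HitStayActors, which Tick loops through to fire stay-hit calls.
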(event EventTick
  (params (DeltaSeconds :type Float%20%28single-precision%29))
  (for _array_element (Variables|Default|GetHitStayActors)
    (Default|CallOnStayHit _array_element)))

(fn InitTargetSMComponent
  (params (TargetSMComponent :type Static%20Mesh%20Component%20Object%20Reference) (AddedSMComponent :type Static%20Mesh%20Component%20Object%20Reference) (EnlargeScale :type Float%20%28double-precision%29))
  (Utilities|FlowControl|Sequence
    (:then_0
      (LocalVariables|SetTargetSMComp TargetSMComponent)
      (bind _output_get (LocalVariables|SetAddedSMComp AddedSMComponent))
      (Transformation|AttachComponentToComponent _output_get (LocalVariables|GetTargetSMComp) "None" "KeepRelative" "KeepRelative" "KeepRelative" true)
      (Collision|SetCollisionEnabled (LocalVariables|GetAddedSMComp) "QueryOnly")
      (Components|StaticMesh|SetStaticMesh (LocalVariables|GetAddedSMComp) (Variables|/Script/Engine.StaticMeshComponent|GetStaticMesh (LocalVariables|GetTargetSMComp)))
      (Transformation|SetRelativeScale3D (LocalVariables|GetAddedSMComp) (Math|Conversions|ToVector(Float) EnlargeScale))
      (Variables|/Script/Engine.PrimitiveComponent|SetbGenerateOverlapEvents (LocalVariables|GetAddedSMComp) true)
      (Collision|SetCollisionResponsetoAllChannels (LocalVariables|GetAddedSMComp) "ECR_Overlap")
      (Variables|Default|SetMyObjectType (Collision|GetCollisionObjectType (LocalVariables|GetAddedSMComp))))
    (:then_1
      (Collision|BindEventtoOnComponentBeginOverlap AddedSMComponent (EventDispatchers|CreateEvent :!event BPSetHitEventsComponentAutoGenFunc))
      (Collision|BindEventtoOnComponentEndOverlap AddedSMComponent (EventDispatchers|CreateEvent :!event BPSetHitEventsComponentAutoGenFunc1)))))

(fn BPSetHitEventsComponentAutoGenFunc
  (params (OverlappedComponent :type Primitive%20Component%20Object%20Reference) (OtherActor :type Actor%20Object%20Reference) (OtherComp :type Primitive%20Component%20Object%20Reference) (OtherBodyIndex :type Integer) (bFromSweep :type Boolean) (SweepResult :type Hit%20Result%20Structure%20%28by%20ref%29))
  (if (Utilities|Enum|Equal(Enum) (Collision|GetCollisionResponsetoChannel OtherComp (Variables|Default|GetMyObjectType)) "ECR_Block")
    (Utilities|Array|Add (Variables|Default|GetHitStayActors) OtherActor)
    (Default|CallOnBeginHit OtherActor)
    (return)))

(fn BPSetHitEventsComponentAutoGenFunc1
  (params (OverlappedComponent :type Primitive%20Component%20Object%20Reference) (OtherActor :type Actor%20Object%20Reference) (OtherComp :type Primitive%20Component%20Object%20Reference) (OtherBodyIndex :type Integer))
  (if (Utilities|Enum|Equal(Enum) (Collision|GetCollisionResponsetoChannel OtherComp (Variables|Default|GetMyObjectType)) "ECR_Block")
    (Utilities|Array|RemoveItem (Variables|Default|GetHitStayActors) OtherActor)
    (Default|CallOnEndHit OtherActor)))